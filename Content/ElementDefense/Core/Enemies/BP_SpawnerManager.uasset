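; BP_SpawnerManager controls enemy spawning across stages, creating enemies of the stage's element types at random spawn points.
; On BeginPlay it caches all BP_SpawnerPoints and creates a paused looping spawn timer.
; NewStage sets the element list and unpauses the timer, whose ticks message a random spawner with a random element.
; EndStage pauses the timer and force-kills every Enemy_Char through the BOOM message.
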(event `self.ReceiveBeginPlay`
  (bind _returnvalue (`KismetSystemLibrary.K2_SetTimer` null "Spawn Enemy" 4.0 true))
  (bind _output_get (set `self.Spawn Enemy Handle` _returnvalue))
  (`KismetSystemLibrary.K2_PauseTimerHandle` _output_get)
  (bind _outactors (`GameplayStatics.GetAllActorsOfClass` "/Game/ElementDefense/Core/Enemies/BP_SpawnerPoints.BP_SpawnerPoints_C"))
  (set `self.Spawner Points` _outactors))

(event `Spawn Enemy`
  (bind _output_get (set `self.Selected Spawner` (`KismetArrayLibrary.Array_Random` (`self.Spawner Points`))))
  (`/Engine/EditorBlueprintResources/StandardMacros.IsValid` _output_get
    (:`Is Valid`
      (message `/Game/ElementDefense/Core/Enemies/BPI_Spawner.Spawn Enemies` (`self.Selected Spawner`) (`KismetArrayLibrary.Array_Random` (`self.Element Type`))))))

(event `/Game/ElementDefense/Core/Enemies/BPI_Spawner.New Stage`
  (params (`Element Type` :type "Array of /Game/ElementDefense/Core/Enemies/E_ElementType Enum (by ref)" :default _))
  (set `self.Element Type` `Element Type`)
  (`KismetSystemLibrary.K2_UnPauseTimerHandle` (`self.Spawn Enemy Handle`)))

(event `/Game/ElementDefense/Core/Enemies/BPI_Spawner.End Stage`
  (`KismetSystemLibrary.K2_PauseTimerHandle` (`self.Spawn Enemy Handle`))
  (bind _outactors (`GameplayStatics.GetAllActorsOfClass` "/Game/ElementDefense/Core/Enemies/Enemy_Char.Enemy_Char_C"))
  (for _array_element _outactors
    (message `/Game/ElementDefense/Core/BPI_Catapult.BOOM` _array_element "NewEnumerator0" true)))

(fn `UserConstructionScript`)