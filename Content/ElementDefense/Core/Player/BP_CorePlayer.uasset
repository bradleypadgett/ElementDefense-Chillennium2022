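; Base player character for ElementDefense, handling movement, camera, interaction, health and HUD, with stubbed death, lives and time hooks.
; Tick adds extra downward force around the jump apex and while falling, and sets spring arm length from a pitch-driven curve.
; A timeline blends sprint speed and FOV, with a looping timer and capsule hits governing sprint state.
; A camera line trace sends InteractMessage to hit actors while grounded.
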(event `self.ReceiveTick`
  (params (DeltaSeconds :type "Float (single-precision)"))
  (`self.Jump Update Gravity`)
  (`self.Update Camera Distance`))

(event `self.ReceiveBeginPlay`
  (bind _returnvalue (`GameplayStatics.GetPlayerCameraManager` 0))
  (set `SceneComponent.bAbsoluteRotation` true (`self.SpringArm`))
  (bind _returnvalue_2 (`|CreateWidget` "/Game/ElementDefense/Core/UI/WBP_Crosshair.WBP_Crosshair_C" (`GameplayStatics.GetPlayerController` 0)))
  (`UserWidget.AddToViewport` _returnvalue_2 0)
  (bind _returnvalue_3 (`|CreateWidget` "/Game/ElementDefense/Core/UI/WBP_Health.WBP_Health_C" (`GameplayStatics.GetPlayerController` 0)))
  (`UserWidget.AddToViewport` _returnvalue_3 0)
  (set `PlayerCameraManager.ViewPitchMin` -85.0 _returnvalue) ; ^ ---
  (set `PlayerCameraManager.ViewPitchMax` 80.0 _returnvalue) ; v ---
)

(event `InputAction|Quit`
  (params (Key :type "Key Structure"))
  (:`Pressed`
    (`KismetSystemLibrary.QuitGame` null "Quit" true)))

(event `InputAxis|Move Forward`
  (params (AxisValue :type "Float (single-precision)"))
  ;[1 1 1 1 36] Walking
  (`self.AddMovementInput` (`self.Get Control Rotation`) AxisValue)
  (if (not (and (> (`self.GetInputAxisValue`) 0.0) (> (`KismetMathLibrary.VSizeSquared` (`self.GetVelocity`)) 0.0)))
    (`self.Set Sprinting` false)))

(event `InputAxis|Look Up`
  (params (AxisValue :type "Float (single-precision)"))
  ;[1 1 1 1 36] Camera
  (`self.AddControllerPitchInput` (* AxisValue (`self.Mouse Sensitivity`))))

(event `InputAxis|Look Up Rate`
  (params (AxisValue :type "Float (single-precision)"))
  ;[1 1 1 1 36] Camera
  (`self.AddControllerPitchInput` (* AxisValue (`GameplayStatics.GetWorldDeltaSeconds`) (`self.Mouse Sensitivity`) 60.0)))

(event `InputAction|Interact`
  (params (Key :type "Key Structure"))
  (bind _returnvalue (`SceneComponent.K2_GetComponentLocation` (`self.Camera`)))
  ;[1 1 1 1 36] Interact
  (:`Pressed`
    (bind _outhit (`KismetSystemLibrary.LineTraceSingle` _returnvalue (+ _returnvalue (* (`KismetMathLibrary.GetForwardVector` (`SceneComponent.K2_GetComponentRotation` (`self.Camera`))) 600.0)) "TraceTypeQuery1" true))
    (bind (_bblockinghit _binitialoverlap _time _distance _location _impactpoint _normal _impactnormal _physmat _hitactor) (`GameplayStatics.BreakHitResult` _outhit))
    (if _bblockinghit
      (if (`NavMovementComponent.IsMovingOnGround` (`self.CharacterMovement`))
        (message `/Game/ElementDefense/Core/BPI_Interact.Interact` _hitactor self)))))

(event `InputAxis|Look Right`
  (params (AxisValue :type "Float (single-precision)"))
  ;[1 1 1 1 36] Camera
  (`self.AddControllerYawInput` (* AxisValue (`self.Mouse Sensitivity`))))

(event `InputAxis|Look Right Rate`
  (params (AxisValue :type "Float (single-precision)"))
  ;[1 1 1 1 36] Camera
  (`self.AddControllerYawInput` (* AxisValue (`GameplayStatics.GetWorldDeltaSeconds`) (`self.Mouse Sensitivity`) 60.0)))

(event `InputAxis|Move Right`
  (params (AxisValue :type "Float (single-precision)"))
  ;[1 1 1 1 36] Walking
  (`self.AddMovementInput` (`.Right Vector` (`self.Get Control Rotation`)) AxisValue))

(event `Update Camera Distance`
  (bind _returnvalue (`GameplayStatics.GetPlayerCameraManager` 0))
  (bind (_returnvalue_roll _returnvalue_pitch) (`KismetMathLibrary.BreakRotator` (`SceneComponent.K2_GetComponentRotation` (`self.Camera`))))
  (bind _returnvalue_2 (`KismetMathLibrary.Abs` (`PlayerCameraManager.ViewPitchMin` _returnvalue)))
  ;[1 1 1 1 36] Camera
  (set `SpringArmComponent.TargetArmLength` (`CurveFloat.GetFloatValue` (`self.Camera Curve`) (/ (+ _returnvalue_pitch _returnvalue_2) (+ _returnvalue_2 (`PlayerCameraManager.ViewPitchMax` _returnvalue)))) (`self.SpringArm`)))

(event `Jump Update Gravity`
  (bind (_returnvalue_x _returnvalue_y _returnvalue_z) (`KismetMathLibrary.BreakVector` (`self.GetVelocity`)))
  ;[1 1 1 1 36] Jumping
  (`/Engine/EditorBlueprintResources/StandardMacros.CompareFloat` 400.0 _returnvalue_z
    (:`>`
      (`CharacterMovementComponent.AddForce` (`self.CharacterMovement`) (`KismetMathLibrary.MakeVector` 0.0 0.0 (`KismetMathLibrary.FClamp` (* -1 (`KismetMathLibrary.Abs` (`KismetMathLibrary.MultiplyMultiply_FloatFloat` _returnvalue_z 2.5))) -500.0))))))

(event `Set Sprinting`
  (params (bSprinting :type Boolean))
  (bind _charactermovement (`self.CharacterMovement`))
  ;[1 1 1 1 36] Sprinting
  (bind _output_get (set `self.bSprinting` bSprinting))
  (if _output_get
    (bind (_direction _alpha) (`Timeline|Sprinting Timeline` :!label _label)
      (:`Update`
        (set `CharacterMovementComponent.MaxWalkSpeed` (`KismetMathLibrary.Lerp` (`self.Walk Speed`) (`self.Sprint Speed`) _alpha) _charactermovement)
        (set `CharacterMovementComponent.MaxWalkSpeedCrouched` (`KismetMathLibrary.Lerp` (`self.Crouch Walk Speed`) 350.0 _alpha) _charactermovement)
        (`CameraComponent.SetFieldOfView` (`self.Camera`) (`KismetMathLibrary.Lerp` 80.0 90.0 _alpha))))
    (else
      (`|ExecutionSequence`
        (:`then_0`
          (goto _label :!via `Reverse`))
        (:`then_1`
          (if (not (`self.bHoldingSprint`))
            (`KismetSystemLibrary.K2_PauseTimer` null "Check Sprint")))))))

(event `Jump Apex`
  ;[1 1 1 1 36] Jumping
)

(event `InputAction|Jump`
  (params (Key :type "Key Structure"))
  ;[1 1 1 1 36] Jumping
  (:`Pressed`
    (add `self.OnReachedJumpApex` (delegate `Jump Apex`))
    (bind _output_get (set `self.bJumping` true))
    (set `CharacterMovementComponent.bNotifyApex` _output_get (`self.CharacterMovement`))
    (`self.Jump`))
  (:`Released`
    (set `self.bJumping` false)
    (`self.StopJumping`)
    (if true
      _)))

(event `InputAction|Sprint`
  (params (Key :type "Key Structure"))
  ;[1 1 1 1 36] Sprinting
  (:`Pressed`
    (set `self.bHoldingSprint` true)
    (`KismetSystemLibrary.K2_SetTimer` null "Check Sprint" 0.05 true)
    (`self.Set Sprinting` true))
  (:`Released`
    (set `self.bHoldingSprint` false)))

(event `Check Sprint`
  ;[1 1 1 1 36] Sprinting
  (if (> (`KismetMathLibrary.VSize` (`self.GetVelocity`)) 0.0)
    (if (`self.bHoldingSprint`)
      (`self.Set Sprinting` true))
    (else
      (`self.Set Sprinting` false)
      (if (not (`self.bHoldingSprint`))
        (`KismetSystemLibrary.K2_PauseTimer` null "Check Sprint")))))

(event `InputAction|Reset`
  (params (Key :type "Key Structure"))
  (:`Pressed`
    (message `/Game/ElementDefense/Core/BPI_Health.Reset Lives` (`GameplayStatics.GetGameInstance`))
    (`GameplayStatics.OpenLevelBySoftObjectPtr` "/Game/BombDefuse/Maps/DemoMap.DemoMap")))

(event `Key|Escape`
  (params (Key :type "Key Structure"))
  (:`Pressed`
    (`KismetSystemLibrary.QuitGame` null "Quit")))

(event `self.CapsuleComponent.OnComponentHit`
  (params (HitComponent :type "PrimitiveComponent Object Reference") (OtherActor :type "Actor Object Reference") (OtherComp :type "PrimitiveComponent Object Reference") (NormalImpulse :type "Vector Structure") (Hit :type "HitResult Structure (by ref)"))
  ;[1 1 1 1 36] Sprinting
  (if (> (+ (`KismetMathLibrary.Abs` (.x (`KismetMathLibrary.GetDirectionUnitVector` (`self.K2_GetActorLocation`) (`.ImpactPoint` (`GameplayStatics.BreakHitResult` Hit))))) (`KismetMathLibrary.Abs` (.y (`KismetMathLibrary.GetDirectionUnitVector` (`self.K2_GetActorLocation`) (`.ImpactPoint` (`GameplayStatics.BreakHitResult` Hit)))))) 0.5)
    (`self.Set Sprinting` false)))

(event `/Game/ElementDefense/Core/BPI_Health.Remove Health`
  (params (Amount :type Integer))
  (bind _output_get (set `self.Health` (`KismetMathLibrary.FClamp` (- (`self.Health`) Amount) 0.0 100.0)))
  (if (`KismetMathLibrary.NearlyEqual_FloatFloat` _output_get 0.0 0.9)
    (`self.Died`)))

(event `Died`)

(fn `Get Health`
  (returns (Health :type "Float (double-precision)"))
  (return (`self.Health`)))

(fn `Get Lives`
  (returns (Lives :type Integer))
  (return 0))

(fn `Get Time`
  (returns (Minutes :type Integer) (Seconds :type Integer))
  (return 0 0))

(fn `UserConstructionScript`)