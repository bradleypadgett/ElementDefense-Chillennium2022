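; Player catapult for Element Defense that charges a shot, previews where it will land and fires a BP_Cannon projectile.
; Charge spawns a BP_Marker and resumes a looping timer that ramps ChargeAmount, tilts the arm and moves the marker to the predicted path's end, with debug drawing.
; Launch pauses the timer, swings the arm back via timeline, then spawns the projectile with that charge and sets the marker to expire.
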(event `self.ReceiveBeginPlay`
  (bind _returnvalue (`KismetSystemLibrary.K2_SetTimer` null "yo" 0.01 true))
  (bind _output_get (set `self.Charge Handle` _returnvalue))
  (`KismetSystemLibrary.K2_PauseTimerHandle` _output_get))

(event `/Game/ElementDefense/Core/BPI_Catapult.Launch`
  (bind _balllocation (`self.BallLocation`))
  (bind _marker (`self.Marker`))
  (`KismetSystemLibrary.K2_PauseTimerHandle` (`self.Charge Handle`))
  (`KismetSystemLibrary.PrintString` (`KismetStringLibrary.Conv_DoubleToString` (`self.ChargeAmount`)))
  (bind (_direction _newtrack_0) (`Timeline|Launch Timeline` :!via `PlayFromStart`)
    (:`Update`
      (`SceneComponent.K2_SetRelativeRotation` (`self.S_Pulter`) (`KismetMathLibrary.MakeRotator` (`KismetMathLibrary.Lerp` (`KismetMathLibrary.Lerp` 0.0 -90.0 (`self.ChargeAmount`)) 0.0 _newtrack_0)) false false))
    (:`Finished`
      (`|SpawnActorFromClass` "/Game/ElementDefense/Core/Player/BP_Cannon.BP_Cannon_C" (`KismetMathLibrary.MakeTransform` (`SceneComponent.K2_GetComponentLocation` _balllocation) (`SceneComponent.K2_GetComponentRotation` _balllocation)) "Undefined" "OverrideRootScale" null (`self.ChargeAmount`) (`self.Velocity Normalized`) null)
      (`/Engine/EditorBlueprintResources/StandardMacros.IsValid` _marker
        (:`Is Valid`
          (`self.SetLifeSpan` _marker 5.0))))))

(event `/Game/ElementDefense/Core/BPI_Catapult.Charge`
  (set `self.ChargeAmount` 0.0)
  (`KismetSystemLibrary.K2_UnPauseTimerHandle` (`self.Charge Handle`))
  (bind _returnvalue (`|SpawnActorFromClass` "/Game/ElementDefense/Core/Player/BP_Marker.BP_Marker_C" (`KismetMathLibrary.MakeTransform` (0.0 0.0 0.0)) "Undefined" "OverrideRootScale" null null))
  (set `self.Marker` _returnvalue))

(event `yo`
  (bind _marker (`self.Marker`))
  (bind _output_get (set `self.ChargeAmount` (`KismetMathLibrary.FClamp` (+ (`self.ChargeAmount`) 0.0075) 0.0 1.0)))
  (`SceneComponent.K2_SetRelativeRotation` (`self.S_Pulter`) (`KismetMathLibrary.MakeRotator` (`KismetMathLibrary.Lerp` 0.0 -90.0 _output_get) 0.0 0.0) false false)
  (bind (_outhit _outpathpositions _outlasttracedestination) (`GameplayStatics.Blueprint_PredictProjectilePath_ByTraceChannel` (`SceneComponent.K2_GetComponentLocation` (`self.BallLocation`)) (* (+ (`self.GetActorRightVector`) (0.0 0.0 0.25)) (`KismetMathLibrary.Lerp` 100.0 5000.0 (`self.ChargeAmount`))) true 10.0 "ECC_WorldDynamic" true (`|MakeArray` self :!type "Actor Object Reference") "ForDuration" 0.01 15.0 5.0))
  (`/Engine/EditorBlueprintResources/StandardMacros.IsValid` _marker
    (:`Is Valid`
      (`self.K2_SetActorLocation` _marker _outlasttracedestination false true))))

(fn `UserConstructionScript`)