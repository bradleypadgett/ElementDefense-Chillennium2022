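; BP_Bomb is a projectile bomb that notifies nearby characters of an explosion when it hits something.
; The construction script feeds its Velocity variable into ProjectileMovement.
; Shortly after BeginPlay, it switches Sphere collision to block all channels and starts a random tumbling spin.
; The first Sphere hit sends BOOMMessage to Characters overlapping the second sphere, Sphere1, then destroys the bomb.
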(event `self.ReceiveBeginPlay`
  (bind _returnvalue (`KismetMathLibrary.RandomFloatInRange` 200.0 400.0))
  (`KismetSystemLibrary.Delay` 0.2)
  (`PrimitiveComponent.SetCollisionResponseToAllChannels` (`self.Sphere`) "ECR_Block")
  (set `RotatingMovementComponent.RotationRate` (`KismetMathLibrary.MakeRotator` _returnvalue _returnvalue _returnvalue) (`self.RotatingMovement`)))

(event `self.Sphere.OnComponentHit`
  (params (HitComponent :type "PrimitiveComponent Object Reference") (OtherActor :type "Actor Object Reference") (OtherComp :type "PrimitiveComponent Object Reference") (NormalImpulse :type "Vector Structure") (Hit :type "HitResult Structure (by ref)"))
  (`/Engine/EditorBlueprintResources/StandardMacros.DoOnce` false
    (:`Completed`
      (for _array_element (`PrimitiveComponent.GetOverlappingActors` (`self.Sphere1`) "/Script/Engine.Character")
        (message `/Game/ElementDefense/Core/BPI_Catapult.BOOM` _array_element "NewEnumerator0" false))
      (`self.K2_DestroyActor`))))

(fn `UserConstructionScript`
  (set `MovementComponent.Velocity` (`self.Velocity`) (`self.ProjectileMovement`)))